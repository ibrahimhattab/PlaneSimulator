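; Drivable airplane pawn that the player character can enter, fly and exit, with crash handling.
; Enter and exit swap possession, input mappings, camera and HUD, hiding and attaching the driver while aboard.
; Enhanced Input feeds throttle to BPCAirplane and steering, pitch, roll and brakes to the vehicle movement component, and toggles a wheel flag.
; Three collision boxes spawn fire on impact; two also disable input and reload the Airplane level.
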(event `EnhancedInput|/Game/Input/Actions/IA_MouseLook`
  (params (ActionValue :type "Vector2D Structure") (ElapsedSeconds :type "Float (double-precision)") (TriggeredSeconds :type "Float (double-precision)") (InputAction :type "InputAction Object Reference" :default "/Game/Input/Actions/IA_MouseLook.IA_MouseLook"))
  ; Move
  (:`Triggered`
    (`self.AddControllerYawInput` ActionValue_X)
    (`self.AddControllerPitchInput` ActionValue_Y)))

(event `EnhancedInput|/Game/Blueprints/Vehicles/Airplane/Input/Actions/IA_AirplaneExit`
  (params (ActionValue :type Boolean) (ElapsedSeconds :type "Float (double-precision)") (TriggeredSeconds :type "Float (double-precision)") (InputAction :type "InputAction Object Reference" :default "/Game/Blueprints/Vehicles/Airplane/Input/Actions/IA_AirplaneExit.IA_AirplaneExit"))
  ; ExitAirplane (E)
  (:`Started`
    (`self.ExitAirplane`)))

(event `EnhancedInput|/Game/Blueprints/Vehicles/Airplane/Input/Actions/IA_AirplaneThrottle`
  (params (ActionValue :type "Float (double-precision)") (ElapsedSeconds :type "Float (double-precision)") (TriggeredSeconds :type "Float (double-precision)") (InputAction :type "InputAction Object Reference" :default "/Game/Blueprints/Vehicles/Airplane/Input/Actions/IA_AirplaneThrottle.IA_AirplaneThrottle"))
  ; Throttle
  (:`Triggered`
    (`/Game/Blueprints/Vehicles/Airplane/Component/BPC_Airplane.SetThrottle` (`self.BPC_Airplane`) ActionValue)))

(event `EnhancedInput|/Game/Blueprints/Vehicles/Airplane/Input/Actions/IA_AirplaneSteeringYaw`
  (params (ActionValue :type "Float (double-precision)") (ElapsedSeconds :type "Float (double-precision)") (TriggeredSeconds :type "Float (double-precision)") (InputAction :type "InputAction Object Reference" :default "/Game/Blueprints/Vehicles/Airplane/Input/Actions/IA_AirplaneSteeringYaw.IA_AirplaneSteeringYaw"))
  (bind _vehiclemovementcomponent (`self.VehicleMovementComponent`))
  ; Steering
  (:`Triggered`
    (`ChaosVehicleMovementComponent.SetSteeringInput` _vehiclemovementcomponent ActionValue)
    (`ChaosVehicleMovementComponent.SetYawInput` _vehiclemovementcomponent ActionValue))
  (:`Completed`
    (`ChaosVehicleMovementComponent.SetSteeringInput` _vehiclemovementcomponent 0.0)
    (`ChaosVehicleMovementComponent.SetYawInput` _vehiclemovementcomponent 0.0)))

(event `EnhancedInput|/Game/Blueprints/Vehicles/Airplane/Input/Actions/IA_AirplaneBrake`
  (params (ActionValue :type Boolean) (ElapsedSeconds :type "Float (double-precision)") (TriggeredSeconds :type "Float (double-precision)") (InputAction :type "InputAction Object Reference" :default "/Game/Blueprints/Vehicles/Airplane/Input/Actions/IA_AirplaneBrake.IA_AirplaneBrake"))
  (bind _vehiclemovementcomponent (`self.VehicleMovementComponent`))
  ; Brakes
  (:`Triggered`
    (`ChaosVehicleMovementComponent.SetBrakeInput` _vehiclemovementcomponent 1.0)
    (set `/Game/Blueprints/Vehicles/Airplane/Component/BPC_Airplane.Throttle` 0.0 (`self.BPC_Airplane`)))
  (:`Completed`
    (`ChaosVehicleMovementComponent.SetBrakeInput` _vehiclemovementcomponent 0.0)))

(event `EnhancedInput|/Game/Blueprints/Vehicles/Airplane/Input/Actions/IA_AirplanePitch`
  (params (ActionValue :type "Float (double-precision)") (ElapsedSeconds :type "Float (double-precision)") (TriggeredSeconds :type "Float (double-precision)") (InputAction :type "InputAction Object Reference" :default "/Game/Blueprints/Vehicles/Airplane/Input/Actions/IA_AirplanePitch.IA_AirplanePitch"))
  (bind _vehiclemovementcomponent (`self.VehicleMovementComponent`))
  ; Pitch
  (:`Triggered`
    (`ChaosVehicleMovementComponent.SetPitchInput` _vehiclemovementcomponent ActionValue))
  (:`Completed`
    (`ChaosVehicleMovementComponent.SetPitchInput` _vehiclemovementcomponent 0.0)))

(event `EnhancedInput|/Game/Blueprints/Vehicles/Airplane/Input/Actions/IA_AirplaneRoll`
  (params (ActionValue :type "Float (double-precision)") (ElapsedSeconds :type "Float (double-precision)") (TriggeredSeconds :type "Float (double-precision)") (InputAction :type "InputAction Object Reference" :default "/Game/Blueprints/Vehicles/Airplane/Input/Actions/IA_AirplaneRoll.IA_AirplaneRoll"))
  (bind _vehiclemovementcomponent (`self.VehicleMovementComponent`))
  ; Roll
  (:`Triggered`
    (`ChaosVehicleMovementComponent.SetRollInput` _vehiclemovementcomponent ActionValue))
  (:`Completed`
    (`ChaosVehicleMovementComponent.SetRollInput` _vehiclemovementcomponent 0.0)))

(event `EnhancedInput|/Game/Blueprints/Vehicles/Airplane/Input/Actions/IA_Wheel`
  (params (ActionValue :type Boolean) (ElapsedSeconds :type "Float (double-precision)") (TriggeredSeconds :type "Float (double-precision)") (InputAction :type "InputAction Object Reference" :default "/Game/Blueprints/Vehicles/Airplane/Input/Actions/IA_Wheel.IA_Wheel"))
  (:`Started`
    (`/Engine/EditorBlueprintResources/StandardMacros.FlipFlop`
      (:`A`
        (set `self.bCloseWheel` true))
      (:`B`
        (set `self.bCloseWheel` false)))))

(event `self.Box2.OnComponentBeginOverlap`
  (params (OverlappedComponent :type "PrimitiveComponent Object Reference") (OtherActor :type "Actor Object Reference") (OtherComp :type "PrimitiveComponent Object Reference") (OtherBodyIndex :type Integer) (bFromSweep :type Boolean) (SweepResult :type "HitResult Structure (by ref)"))
  (if (not (or (`GameplayStatics.ObjectIsA` OtherActor "/Game/ThirdPerson/Blueprints/BP_ThirdPersonCharacter.BP_ThirdPersonCharacter_C") (`GameplayStatics.ObjectIsA` OtherActor "BP_Airplane_C")))
    (`NiagaraFunctionLibrary.SpawnSystemAttached` "/Game/Vefects/Free_Fire/Shared/Particles/NS_Fire_Big.NS_Fire_Big" (`self.Box2`) "None" (`.Location` (`GameplayStatics.BreakHitResult` SweepResult)) (struct) "KeepRelativeOffset" true)))

(event `self.Box1.OnComponentBeginOverlap`
  (params (OverlappedComponent :type "PrimitiveComponent Object Reference") (OtherActor :type "Actor Object Reference") (OtherComp :type "PrimitiveComponent Object Reference") (OtherBodyIndex :type Integer) (bFromSweep :type Boolean) (SweepResult :type "HitResult Structure (by ref)"))
  (if (not (or (`GameplayStatics.ObjectIsA` OtherActor "/Game/ThirdPerson/Blueprints/BP_ThirdPersonCharacter.BP_ThirdPersonCharacter_C") (`GameplayStatics.ObjectIsA` OtherActor "BP_Airplane_C")))
    (`NiagaraFunctionLibrary.SpawnSystemAttached` "/Game/Vefects/Free_Fire/Shared/Particles/NS_Fire_Big.NS_Fire_Big" (`self.Box1`) "None" (`.Location` (`GameplayStatics.BreakHitResult` SweepResult)) (struct) "KeepRelativeOffset" true)
    (`self.DisableInput` (`GameplayStatics.GetPlayerController` 0) :!label _label)
    (`KismetSystemLibrary.Delay` 1.5)
    (`GameplayStatics.OpenLevel` "Airplane")))

(event `self.Box.OnComponentBeginOverlap`
  (params (OverlappedComponent :type "PrimitiveComponent Object Reference") (OtherActor :type "Actor Object Reference") (OtherComp :type "PrimitiveComponent Object Reference") (OtherBodyIndex :type Integer) (bFromSweep :type Boolean) (SweepResult :type "HitResult Structure (by ref)"))
  (if (not (or (`GameplayStatics.ObjectIsA` OtherActor "/Game/ThirdPerson/Blueprints/BP_ThirdPersonCharacter.BP_ThirdPersonCharacter_C") (`GameplayStatics.ObjectIsA` OtherActor "BP_Airplane_C")))
    (`NiagaraFunctionLibrary.SpawnSystemAttached` "/Game/Vefects/Free_Fire/Shared/Particles/NS_Fire_Big.NS_Fire_Big" (`self.Box`) "None" (`.Location` (`GameplayStatics.BreakHitResult` SweepResult)) (struct) "KeepRelativeOffset" true)
    (goto _label)))

(fn `CloseHUD`
  (bind _airplanehud (`self.AirplaneHUD`)
    (:`then`
      (`Widget.RemoveFromParent` _airplanehud))
    (:`else`)))

(fn `EnterAirplane`
  (bind _returnvalue (`GameplayStatics.GetPlayerController` 0))
  (bind _currdriver (`self.CurrDriver`))
  ; Enter Airplane
  (bind _output_get (set `self.CurrDriver` (`GameplayStatics.GetPlayerCharacter` 0)))
  (`self.K2_AttachToActor` _output_get self "None" "SnapToTarget" "SnapToTarget" "KeepWorld" true)
  (`PrimitiveComponent.SetCollisionEnabled` (`Character.CapsuleComponent` _currdriver) "NoCollision")
  (`SceneComponent.SetVisibility` (`Character.Mesh` _currdriver) false true)
  (`CharacterMovementComponent.SetMovementMode` (`Character.CharacterMovement` _currdriver) "MOVE_Flying" 0)
  (`Controller.Possess` _returnvalue self)
  (bind _asbp_third_person_player_controller (cast `/Game/ThirdPerson/Blueprints/BP_ThirdPersonPlayerController` _returnvalue))
  (`/Game/ThirdPerson/Blueprints/BP_ThirdPersonPlayerController.Event Add Input Mapping` _asbp_third_person_player_controller "/Game/Blueprints/Vehicles/Airplane/Input/IMC_AirPlane.IMC_AirPlane" 0)
  (`/Game/ThirdPerson/Blueprints/BP_ThirdPersonPlayerController.Event Remove Input Mapping` _asbp_third_person_player_controller "/Game/Input/IMC_Default.IMC_Default")
  (`PlayerController.SetViewTargetWithBlend` _returnvalue self 0.7 "VTBlend_Linear" 0.0 true)
  (`self.OpenHUD`))

(fn `ExitAirplane`
  (bind _returnvalue (`GameplayStatics.GetPlayerController` 0))
  (bind _currdriver (`self.CurrDriver`))
  (`self.K2_DetachFromActor` _currdriver "KeepRelative" "KeepRelative" "KeepWorld")
  (`self.K2_SetActorLocation` _currdriver (`SceneComponent.K2_GetComponentLocation` (`self.ExitPlayer`)) false false)
  (`PrimitiveComponent.SetCollisionEnabled` (`Character.CapsuleComponent` _currdriver) "QueryAndPhysics")
  (`SceneComponent.SetVisibility` (`Character.Mesh` _currdriver) true true)
  (`Controller.Possess` _returnvalue (`self.CurrDriver`))
  (bind _asbp_third_person_player_controller (cast `/Game/ThirdPerson/Blueprints/BP_ThirdPersonPlayerController` _returnvalue))
  (`/Game/ThirdPerson/Blueprints/BP_ThirdPersonPlayerController.Event Add Input Mapping` _asbp_third_person_player_controller "/Game/Input/IMC_Default.IMC_Default" 0)
  (`/Game/ThirdPerson/Blueprints/BP_ThirdPersonPlayerController.Event Remove Input Mapping` _asbp_third_person_player_controller "/Game/Blueprints/Vehicles/Airplane/Input/IMC_AirPlane.IMC_AirPlane")
  (`PlayerController.SetViewTargetWithBlend` _returnvalue (`self.CurrDriver`) 0.7 "VTBlend_Linear" 0.0 true)
  (`self.CloseHUD`))

(fn `GetAirplaneMesh`
  (returns (AirplaneMesh :type "SkeletalMeshComponent Object Reference"))
  (return (`self.Mesh`)))

(fn `OpenHUD`
  (bind _returnvalue (`|CreateWidget` "/Game/Blueprints/Vehicles/Airplane/UI/WB_AirplaneHUD.WB_AirplaneHUD_C" (`GameplayStatics.GetPlayerController` 0) null))
  (set `self.AirplaneHUD` _returnvalue)
  (`UserWidget.AddToViewport` _returnvalue 0))

(fn `UserConstructionScript`)