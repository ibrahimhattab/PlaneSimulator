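; Airplane flight physics component that drives the owner's mesh with thrust, lift and drag forces.
; Each tick it caches mesh state, then applies thrust from working engines, curve-scaled capped lift from intact surfaces, and throttle-blended drag.
; All forces act at center of mass, and angle of attack comes from nose angle against the horizon, not airflow.
; It also exposes stepped throttle control and a flight telemetry struct.
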(event `self.ReceiveBeginPlay`
  (bind _airplanemesh (message `/Game/Blueprints/Vehicles/Airplane/Interface/BPI_Airplane.GetAirplaneMesh` (`self.GetOwner`)))
  (set `self.AirplaneMesh` _airplanemesh)
  (`self.CalculateMaxLiftForce`))

(event `self.ReceiveTick`
  (params (DeltaSeconds :type "Float (single-precision)"))
  (`|ExecutionSequence`
    (:`then_0`
      (`self.SetAirplaneVeriables`))
    (:`then_1`
      (`self.ApplyThrust`)
      (`self.CalculateAOA`)
      (`self.ApplyLift`)
      (`self.ApplyDrag`))))

(fn `ApplyDrag`
  (bind _returnvalue (* (* (* (`self.AirplaneVelocity`) -1.0) (`KismetMathLibrary.MultiplyMultiply_FloatFloat` (`self.SpeedMPS`) 2.0)) (`KismetMathLibrary.Lerp` (`self.MinDragCoffecient`) (`self.MaxDragCoffecient`) (`self.Throttle`))))
  (set `self.DragForce` (`KismetMathLibrary.VSize` _returnvalue))
  (`PrimitiveComponent.AddForceAtLocation` (`self.AirplaneMesh`) _returnvalue (`self.COM`) "None"))

(fn `ApplyLift`
  (`self.AirplaneMesh`
    (:`then`
      (for _array_element (`self.Surfaces`)
        (bind (_surfacetype _surfacelocation _liftmultiplier _lifeefficiencycurve _bsurfacebroken) (break `/Game/Blueprints/Vehicles/Airplane/Data/Structures/F_AirplaneSurfaces` _array_element))
        (if (not _bsurfacebroken)
          (bind _liftforce (`self.CalculateLiftForce` _liftmultiplier _lifeefficiencycurve))
          (bind _returnvalue (* _liftforce (`SceneComponent.GetUpVector` (`self.AirplaneMesh`))))
          (set `self.LiftForce` (`KismetMathLibrary.VSize` _returnvalue))
          (`PrimitiveComponent.AddForceAtLocation` (`self.AirplaneMesh`) _returnvalue (`self.COM`) "None"))))
    (:`else`)))

(fn `ApplyThrust`
  (`self.AirplaneMesh`
    (:`then`
      (for _array_element (`self.Engines`)
        (bind (_acceleration _enginelocation _benginebroken _bengineon) (break `/Game/Blueprints/Vehicles/Airplane/Data/Structures/F_AirplaneEngine` _array_element))
        (if _bengineon
          (if (not _benginebroken)
            (bind _thrustforce (`self.CalculateThrustForce` _acceleration))
            (bind _returnvalue (* _thrustforce (`SceneComponent.GetForwardVector` (`self.AirplaneMesh`)) (`self.Throttle`)))
            (set `self.ThurstForce` (`KismetMathLibrary.VSize` _returnvalue))
            (`PrimitiveComponent.AddForceAtLocation` (`self.AirplaneMesh`) _returnvalue (`self.COM`) "None")))))
    (:`else`)))

(fn `CalculateAOA`
  ; If the Plane's nose is up it'll give positive, and if it's down it'll give negative
  (bind _airplanemesh (`self.AirplaneMesh`)
    (:`then`
      (bind (_returnvalue_x _returnvalue_y) (`KismetMathLibrary.BreakVector` (`SceneComponent.GetForwardVector` _airplanemesh)))
      (bind _returnvalue (`KismetMathLibrary.DegAcos` (`KismetMathLibrary.Dot_VectorVector` (`SceneComponent.GetForwardVector` _airplanemesh) (`KismetMathLibrary.MakeVector` _returnvalue_x _returnvalue_y))))
      (set `self.AOA` (`KismetMathLibrary.SelectFloat` _returnvalue (* _returnvalue -1.0) (> (`self.Pitch`) 0.0))))
    (:`else`)))

(fn `CalculateLiftForce`
  (params (LiftMultiplier :type "Float (double-precision)") (LiftEfficiencyCurve :type "CurveFloat Object Reference"))
  (returns (LiftForce :type "Float (double-precision)"))
  (return (* (`KismetMathLibrary.FClamp` (* LiftMultiplier (/ (`KismetMathLibrary.MultiplyMultiply_FloatFloat` (`self.SpeedCMPS`) 2.0) 2.0)) 0.0 (`self.MaxLiftForce`)) (`CurveFloat.GetFloatValue` (`local.LiftEfficiencyCurve`) (`self.AOA`)))))

(fn `CalculateMaxLiftForce`
  (bind _airplanemesh (`self.AirplaneMesh`)
    (:`then`
      (set `self.MaxLiftForce` (* (`PrimitiveComponent.GetMass` _airplanemesh) (`self.MaxLiftAcceleration`) 100.0)))
    (:`else`)))

(fn `CalculateThrustForce`
  (params (Acceleration :type "Float (double-precision)"))
  (returns (ThrustForce :type "Float (double-precision)"))
  (return (* Acceleration (`PrimitiveComponent.GetMass` (`self.AirplaneMesh`)) 100.0)))

(fn `GetInfos`
  (returns (AirplaneInfos :type "/Game/Blueprints/Vehicles/Airplane/Data/Structures/F_AirplaneInfos Structure"))
  (return (make `/Game/Blueprints/Vehicles/Airplane/Data/Structures/F_AirplaneInfos` (`self.AirplaneAltitudeMeters`) (`self.AOA`) (`self.DragForce`) (`self.LiftForce`) (`self.Pitch`) (`self.SpeedCMPS`) (`self.SpeedMPS`) (`self.Throttle`) (`self.ThurstForce`))))

(fn `SetAirplaneVeriables`
  (bind (_returnvalue_roll _returnvalue_pitch) (`KismetMathLibrary.BreakRotator` (`SceneComponent.K2_GetComponentRotation` (`self.AirplaneMesh`))))
  (bind _returnvalue (`SceneComponent.GetComponentVelocity` (`self.AirplaneMesh`)))
  (bind (_returnvalue_x _returnvalue_y _returnvalue_z) (`KismetMathLibrary.BreakVector` (`SceneComponent.K2_GetComponentLocation` (`self.AirplaneMesh`))))
  (`self.AirplaneMesh`
    (:`then`
      (`|ExecutionSequence`
        (:`then_0`
          (set `self.COM` (`SkeletalMeshComponent.GetSkeletalCenterOfMass` (`self.AirplaneMesh`)))
          (set `self.SpeedMPS` (/ (`KismetMathLibrary.VSizeXY` (`SceneComponent.GetComponentVelocity` (`self.AirplaneMesh`))) 100.0)))
        (:`then_1`
          (set `self.Pitch` _returnvalue_pitch)
          (set `self.AirplaneAltitudeMeters` (/ _returnvalue_z 100.0)))
        (:`then_2`
          (set `self.SpeedCMPS` (`KismetMathLibrary.VSizeXY` _returnvalue))
          (set `self.AirplaneVelocity` _returnvalue))))
    (:`else`)))

(fn `SetThrottle`
  (params (ThrottleInput :type "Float (double-precision)"))
  (if (> ThrottleInput 0.0)
    (set `self.Throttle` (`KismetMathLibrary.FClamp` (+ (`self.Throttle`) (`self.ThrottleStep`))))
    (else
      (set `self.Throttle` (`KismetMathLibrary.FClamp` (- (`self.Throttle`) (`self.ThrottleStep`)))))))